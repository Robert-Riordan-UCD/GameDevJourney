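; Enemy manager for the SpaceShooter game that spawns BP_Enemy AI pawns around itself, up to a MaxEnemies cap.
; A looping timer started on BeginPlay spawns each enemy at SpawnRadius from the root in a random 3D direction and tracks it in an array.
; At the cap, it removes invalid entries while iterating that array and immediately rechecks, which loops endlessly if all enemies remain valid.
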(event Custom|SpawnEnemy
  ;[1 1 1] Spawn timer
  ;[1 1 1] Check if enemy can be spawned
  (if (< (Utilities|Array|Length (Variables|Default|GetEnemies)) (Variables|Default|GetMaxEnemies)) :!label _label
    ;[1 1 1] Spawn new enemy
    (bind _location (CallFunction|GetRandomSpawnLocation))
    (bind _returnvalue (AI|SpawnAIFromClass "/Game/SpaceShooter/Blueprints/BP_Enemy.BP_Enemy_C" 0 _location "0, 0, 0" false 0))
    (Utilities|Array|Add (Variables|Default|GetEnemies) _returnvalue)
    (else
      ;[1 1 1] Remove dead enemies
      (for _array_element (Variables|Default|GetEnemies)
        (if (not (Utilities|IsValid _array_element))
          (Utilities|Array|RemoveItem (Variables|Default|GetEnemies) _array_element)))
      (goto _label))))

(event EventBeginPlay
  ;[1 1 1] Spawn timer
  (Utilities|Time|SetTimerbyEvent (delegate Custom|SpawnEnemy) (Variables|Default|GetSpawnRate) true))

(fn ConstructionScript)

(fn GetRandomSpawnLocation
  (return (+ (Transformation|GetWorldLocation (Variables|Default|GetDefaultSceneRoot)) (* (Math|Random|RandomUnitVector) (Variables|Default|GetSpawnRadius)))))