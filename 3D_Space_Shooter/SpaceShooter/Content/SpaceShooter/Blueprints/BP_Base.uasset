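; BP_Base is a space shooter Blueprint that gives an actor health and team-based damage handling.
; Its TakeDamage event receives a damage amount and a team, and subtracts the damage from Health only when that team differs from its own.
; The actor destroys itself when Health reaches zero or below, and otherwise prints the remaining Health.
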(event EventBeginPlay)

(event Collision|EventActorBeginOverlap
  (params (OtherActor :type Actor%20Object%20Reference)))

(event EventTick
  (params (DeltaSeconds :type Float%20%28single-precision%29)))

(event EventTakeDamage
  (params (Damage :type Float%20%28double-precision%29) (Team :type E_Team%20Enum :default "NewEnumerator0"))
  ;[1 1 1] Take damage
  (if (Utilities|Enum|NotEqual(Enum) Team (Variables|Default|GetTeam))
    (bind _output_get (Variables|Default|SetHealth (- (Variables|Default|GetHealth) Damage)))
    ;[1 1 1] Die
    (if (<= _output_get 0.0)
      (Actor|DestroyActor)
      (else
        (Development|PrintString (Utilities|String|ToString(Float) _output_get))))))

(fn ConstructionScript)