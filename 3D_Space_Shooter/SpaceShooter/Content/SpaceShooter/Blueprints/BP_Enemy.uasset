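; Enemy pawn for a space shooter that chases the player, registering itself with the player on BeginPlay via a message call.
; One looping timer periodically picks a random 3D offset around the player, so the pursuit point wanders.
; A faster timer reads the player's position, then interpolates rotation and FloatingPawnMovement velocity toward that offset point at max speed.
; Velocity and location are debug-printed; EnemyCommand and GetPawnInfo are empty stubs.
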(event Custom|Generate%20Random%20Offset%20Tick
  (Variables|RandomOffset|SetRandomOffset (CallFunction|GenerateRandomOffeset)))

(event Custom|Velocity%20Update%20Tick
  (bind _floatingpawnmovement (Variables|Default|GetFloatingPawnMovement))
  (bind _position (Class|BPIEnemy|GetPawnInfo(Message) (Variables|Base|GetPlayer)))
  (Utilities|FlowControl|Sequence
    (:then_0
      ;[1 1 1] Face same direction as player?
      (Transformation|SetActorRotation (Math|Interpolation|RInterpTo (Transformation|GetActorRotation) (Math|Conversions|RotationFromXVector (Math|Vector|Normalize (- (+ _position (Variables|RandomOffset|GetRandomOffset)) (Transformation|GetActorLocation)))) 0.05 1e+01)))
    (:then_1
      ;[1 1 1] Set Velocity
      (bind _output_get (Variables|/Script/Engine.MovementComponent|SetVelocity _floatingpawnmovement (Math|Interpolation|VInterpTo (Variables|/Script/Engine.MovementComponent|GetVelocity _floatingpawnmovement) (* (Math|Vector|Normalize (- (+ _position (Variables|RandomOffset|GetRandomOffset)) (Transformation|GetActorLocation))) (Variables|Movement|GetMaxSpeed)) 0.05 1e+01)))
      (Development|PrintString (Utilities|String|ToString(Vector) _output_get))
      (Development|PrintString (Utilities|String|ToString(Vector) (Transformation|GetActorLocation self)) true true "(R=0.639179,G=0.000000,B=1.000000,A=1.000000)"))))

(event EventEnemyCommand
  (params (New%20State :type E_Enemy_State%20Enum :default "NewEnumerator0")))

(event EventBeginPlay
  (bind _output_get (Variables|Base|SetPlayer (Game|Player|GetPlayerPawn 0)))
  (Utilities|IsValid _output_get
    (:Is%20Valid
      (Class|BPIEnemy|EnemyAdd(Message) _output_get self)
      (bind _returnvalue (Utilities|Time|SetTimerbyEvent (delegate Custom|Generate%20Random%20Offset%20Tick) 0.5 true))
      (Variables|RandomOffset|SetRandomOffsetTimer _returnvalue)
      (Utilities|Time|SetTimerbyEvent (delegate Custom|Velocity%20Update%20Tick) 0.05 true))
    (:Is%20Not%20Valid
      (Development|PrintString "No valid player found by enemy"))))

(fn ConstructionScript)

(fn GenerateRandomOffeset
  (bind _randomoffsetminmax (Variables|RandomOffset|GetRandomOffsetMinMax))
  (bind _randomoffsetminmax_2 (Variables|RandomOffset|GetRandomOffsetMinMax))
  (bind _randomoffsetminmax_3 (Variables|RandomOffset|GetRandomOffsetMinMax))
  (return (Math|Vector|MakeVector (Math|Random|RandomFloatinRange (* -1.0 _randomoffsetminmax_2) _randomoffsetminmax_2) (Math|Random|RandomFloatinRange (* -1.0 _randomoffsetminmax_3) _randomoffsetminmax_3) (Math|Random|RandomFloatinRange (* -1.0 _randomoffsetminmax) _randomoffsetminmax))))

(fn GetPawnInfo
  (return "0, 0, 0" "0, 0, 0" 0.0))