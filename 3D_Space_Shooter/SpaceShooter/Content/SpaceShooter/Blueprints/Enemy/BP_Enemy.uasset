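; Enemy ship pawn for the space shooter that pursues the player or attacks a base, and is destroyed when its health runs out.
; A Tick-driven state machine steers with interpolated velocity and random offsets, facing the direction of travel.
; Nearing the player triggers a timed idle before pursuit resumes.
; A blocked line trace switches to following a flight path requested from the base, currently without weapon fire, then idling.
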(event Custom|StopIdleFly
  ;[1 1 1] Return to persuit
  (CallFunction|ChangeState "NewEnumerator0")
  ;[1 1 1] Update random offset
  (Variables|RandomOffset|SetRandomOffset (CallFunction|GenerateRandomOffeset)))

(event EventSetBase
  (params (Base :type BP%20Base%20Object%20Reference))
  ;[1 1 1] Set base
  (Variables|Default|SetBase Base))

(event EventTick
  (params (DeltaSeconds :type Float%20%28single-precision%29))
  (bind _returnvalue (Transformation|GetActorLocation))
  (bind _floatingpawnmovement (Variables|Default|GetFloatingPawnMovement))
  (bind _floatingpawnmovement_2 (Variables|Default|GetFloatingPawnMovement))
  (Utilities|FlowControl|Sequence
    (:then_0
      (switch Utilities|FlowControl|Switch|SwitchonE_Enemy_State (Variables|State|GetCurrentState)
        (:NewEnumerator0
          (bind _position (Class|BPIEnemy|GetPawnInfo(Message) (Variables|Base|GetPlayer)))
          (Utilities|FlowControl|Sequence
            (:then_1
              ;[1 1 1] Set Velocity
              (Variables|/Script/Engine.MovementComponent|SetVelocity _floatingpawnmovement (Math|Interpolation|VInterpTo (Variables|/Script/Engine.MovementComponent|GetVelocity _floatingpawnmovement) (* (Math|Vector|Normalize (- (+ _position (Variables|RandomOffset|GetRandomOffset)) (Transformation|GetActorLocation))) (Variables|Movement|GetMaxSpeed)) 0.05 1e+01)))
            (:then_2
              ;[1 1 1] Near player stop persuing
              (if (< (Math|Vector|VectorLength (- _position (Transformation|GetActorLocation))) (Variables|State|GetNearTargetThreshold))
                (CallFunction|ChangeState "NewEnumerator2")
                ;[1 1 1] Return to persuit
                (Utilities|Time|SetTimerbyEvent (delegate Custom|StopIdleFly) (Variables|State|GetIdleTime))))
            (:then_3
              ;[1 1 1] Can't see player. Switch to attacking base
              (bind (_outhit _returnvalue_2) (Collision|LineTraceForObjects (Transformation|GetWorldLocation (Variables|Default|GetDefaultSceneRoot)) _position (Variables|State|GetObject%20Types) false 0 "None"))
              (if _returnvalue_2
                (if (!= (Actor|GetComponentbyClass (.HitActor (Collision|BreakHitResult _outhit)) "/Script/Engine.ActorComponent") "/Game/SpaceShooter/Blueprints/PlayerSpaceShip.PlayerSpaceShip")
                  (CallFunction|ChangeState "NewEnumerator1"))))))
        (:NewEnumerator1
          (if (> (Utilities|Array|Length (Variables|Default|GetFlightPath)) 0)
            ;[1 1 1] Set Velocity
            (Variables|/Script/Engine.MovementComponent|SetVelocity _floatingpawnmovement_2 (Math|Interpolation|VInterpTo (Variables|/Script/Engine.MovementComponent|GetVelocity _floatingpawnmovement_2) (* (Math|Vector|Normalize (- (+ (Utilities|Array|Get(acopy) (Variables|Default|GetFlightPath)) (Variables|RandomOffset|GetRandomOffset)) (Transformation|GetActorLocation))) (Variables|Movement|GetMaxSpeed)) 0.05 1e+01))
            (if (< (Math|Vector|VectorLength (- (Utilities|Array|Get(acopy) (Variables|Default|GetFlightPath)) (Transformation|GetWorldLocation (Variables|Default|GetDefaultSceneRoot)))) (Variables|State|GetNearTargetThreshold))
              (Utilities|Array|RemoveIndex (Variables|Default|GetFlightPath))
              (else
                (Development|PrintString "Attacking base")))
            (else
              (CallFunction|ChangeState "NewEnumerator2"))))))
    (:then_1
      ;[1 1 1] Face in direction of movement
      (Transformation|SetActorRotation (Math|Interpolation|RInterpTo (Transformation|GetActorRotation) (Math|Rotator|FindLookatRotation _returnvalue (+ _returnvalue (Transformation|GetVelocity))) 0.05 1e+01)))))

(event EventBeginPlay
  ;[1 1 1] Get player info
  (bind _output_get (Variables|Base|SetPlayer (Game|Player|GetPlayerPawn 0)))
  (Utilities|IsValid _output_get
    (:Is%20Valid
      (Class|BPIEnemy|EnemyAdd(Message) _output_get self))))

(event EventTakeDamage
  (params (Damage :type Float%20%28double-precision%29) (Team :type E_Team%20Enum :default "NewEnumerator0"))
  ;[1 1 1] Take damage
  (if (Utilities|Enum|NotEqual(Enum) Team (Variables|Default|GetTeam))
    (bind _output_get (Variables|Base|SetHealth (- (Variables|Base|GetHealth) Damage)))
    ;[1 1 1] Die
    (if (<= _output_get 0.0)
      (Actor|DestroyActor))))

(fn ConstructionScript)

(fn GenerateRandomOffeset
  (bind _randomoffsetminmax (Variables|RandomOffset|GetRandomOffsetMinMax))
  (bind _randomoffsetminmax_2 (Variables|RandomOffset|GetRandomOffsetMinMax))
  (bind _randomoffsetminmax_3 (Variables|RandomOffset|GetRandomOffsetMinMax))
  (return (Math|Vector|MakeVector (Math|Random|RandomFloatinRange (* -1.0 _randomoffsetminmax_2) _randomoffsetminmax_2) (Math|Random|RandomFloatinRange (* -1.0 _randomoffsetminmax_3) _randomoffsetminmax_3) (Math|Random|RandomFloatinRange (* -1.0 _randomoffsetminmax) _randomoffsetminmax))))

(fn ChangeState
  (params (NewState :type E_Enemy_State%20Enum :default "NewEnumerator0"))
  (if (not (Utilities|Enum|Equal(Enum) NewState (Variables|State|GetCurrentState)))
    (bind _output_get (Variables|State|SetCurrentState NewState))
    (switch Utilities|FlowControl|Switch|SwitchonE_Enemy_State _output_get
      (:NewEnumerator1
        (bind _flightpath (Class|BPIRequestFlightPath|RequestFlightPath(Message) (Variables|Default|GetBase) (Transformation|GetWorldLocation (Variables|Default|GetDefaultSceneRoot))))
        (Variables|Default|SetFlightPath _flightpath)))))

(fn GetPawnInfo
  (return "0, 0, 0" "0, 0, 0" 0.0))