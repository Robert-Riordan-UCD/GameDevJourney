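; BP_Base is a team base in a space shooter that can be destroyed and hands out flight paths.
; TakeDamage ignores hits from its own team, subtracts damage from Health, then destroys the actor at zero or prints the remaining health.
; RequestFlightPath builds a path from the NavPoint nearest the given position, followed by that point mirrored by negating its Y coordinate.
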(event EventBeginPlay)

(event Collision|EventActorBeginOverlap
  (params (OtherActor :type Actor%20Object%20Reference)))

(event EventTick
  (params (DeltaSeconds :type Float%20%28single-precision%29)))

(event EventTakeDamage
  (params (Damage :type Float%20%28double-precision%29) (Team :type E_Team%20Enum :default "NewEnumerator0"))
  ;[1 1 1] Take damage
  (if (Utilities|Enum|NotEqual(Enum) Team (Variables|Default|GetTeam))
    (bind _output_get (Variables|Default|SetHealth (- (Variables|Default|GetHealth) Damage)))
    ;[1 1 1] Die
    (if (<= _output_get 0.0)
      (Actor|DestroyActor)
      (else
        (Development|PrintString (Utilities|String|ToString(Float) _output_get))))))

(fn ConstructionScript)

(fn GetNearestNavPoint
  (params (Position :type Vector))
  (LocalVariables|SetNearestPoint (Utilities|Array|Get(acopy) (Variables|Default|GetNavPoints)))
  (for _array_element (Variables|Default|GetNavPoints)
    (if (< (Math|Vector|VectorLength (- _array_element Position)) (Math|Vector|VectorLength (- Position (LocalVariables|GetNearestPoint))))
      (LocalVariables|SetNearestPoint _array_element)))
  (return (LocalVariables|GetNearestPoint)))

(fn RequestFlightPath
  (params (CurrentPosition :type Vector :default "0, 0, 0"))
  (bind _point (CallFunction|GetNearestNavPoint CurrentPosition))
  (Utilities|Array|Add (LocalVariables|GetPath) _point)
  (Utilities|Array|Add (LocalVariables|GetPath) (* _point "1.000000,-1.000000,1.000000"))
  (return (LocalVariables|GetPath)))